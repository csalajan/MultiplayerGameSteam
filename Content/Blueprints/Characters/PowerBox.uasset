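; Player-owned power box that carries a health pool, kills its owner's character when damage depletes it, and can be picked back up outside combat.
; A timeline polls owner distance, starting a looping timer that drains health and flashes the owner's screen while out of range.
; Damage from others applies on authority, with RepNotify updating a floating health bar that a second timeline turns toward the player.
; Box overlap enables F-key pickup, returning remaining health.
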(event OnComponentBeginOverlap(Box)
  (params (OverlappedComponent :type Primitive%20Component%20Object%20Reference) (OtherActor :type Actor%20Object%20Reference) (OtherComp :type Primitive%20Component%20Object%20Reference) (OtherBodyIndex :type Integer) (bFromSweep :type Boolean) (SweepResult :type Hit%20Result%20Structure%20%28by%20ref%29))
  ;[1 1 1 1 32] Enable Input
  (if (== OtherActor (Variables|Default|GetOwningPlayer))
    (Input|EnableInput (Game|GetPlayerController 0))))

(event OnComponentEndOverlap(Box)
  (params (OverlappedComponent :type Primitive%20Component%20Object%20Reference) (OtherActor :type Actor%20Object%20Reference) (OtherComp :type Primitive%20Component%20Object%20Reference) (OtherBodyIndex :type Integer))
  ;[1 1 1 1 32] Enable Input
  (if (== OtherActor (Variables|Default|GetOwningPlayer))
    (Input|DisableInput (Game|GetPlayerController 0))))

(event OnComponentHit(Cube)
  (params (HitComponent :type Primitive%20Component%20Object%20Reference) (OtherActor :type Actor%20Object%20Reference) (OtherComp :type Primitive%20Component%20Object%20Reference) (NormalImpulse :type Vector :default "0, 0, 0") (Hit :type Hit%20Result%20Structure%20%28by%20ref%29))
  (Physics|SetSimulatePhysics (Variables|Default|GetCube) false))

(event Custom|SetValues
  (params (HealthFromCharacter :type Float%20%28single-precision%29))
  ;[1 1 1 1 32] Set Health Value and owning player
  (bind _output_get (Variables|Default|SetPowerBoxHealth HealthFromCharacter))
  (Development|PrintString (Utilities|String|ToString(Float) _output_get) true true "(R=1.000000,G=0.090672,B=0.000000,A=1.000000)"))

(event Custom|CheckPlayerDistance
  ;[1 1 1 1 32] If Player is out of range - deal damage to player
  (Timeline|CheckPlayerInRange Play
    (:Update
      (if (> (Transformation|GetDistanceTo (Variables|Default|GetOwningPlayer)) 1.3e+03)
        (Utilities|FlowControl|DoOnce false
          (:Completed
            (Variables|Default|SetPlayerOutOfRange true)
            (Development|PrintString "OutOfRange")
            (bind _returnvalue (Utilities|Time|SetTimerbyEvent (delegate Custom|OutOfRangeDamage) 1.0 true))))
        (elif (Variables|Default|GetPlayerOutOfRange)
          (Variables|Default|SetPlayerOutOfRange false)
          (Utilities|Time|ClearandInvalidateTimerbyHandle _returnvalue)
          (CallFunction|Reset)
          (Development|PrintString "InRange"))))))

(event Custom|HealthBarRotation
  ;[1 1 1 1 32] Update Health Bar Rotation
  (Timeline|WidgetRotation Play
    (:Update
      (Transformation|SetWorldRotation (Variables|Default|GetFloatingHealthBarLoc) (Math|Rotator|FindLookatRotation (Transformation|GetWorldLocation (Variables|Default|GetFloatingHealthBarLoc)) (Class|PlayerController|GetFocalLocation (Game|GetPlayerController 0))) false false))))

(event Custom|Reset
  ;[1 1 1 1 32] If Player is out of range - deal damage to player
  (Utilities|FlowControl|DoOnce false) ; enters at Reset
)

(event Custom|DeathEvent
  ;[1 1 1 1 32] Death Event
  (bind _asthird_person_character (Utilities|Casting|CastToThirdPersonCharacter (Variables|Default|GetOwningPlayer)))
  (Default|DeathEvent _asthird_person_character))

(event Custom|ReturnToPlayer
  ;[1 1 1 1 32] Return Power Box To Player
  (bind _asthird_person_character (Utilities|Casting|CastToThirdPersonCharacter (Game|GetPlayerCharacter 0)))
  (Default|PickUpBox _asthird_person_character (Variables|Default|GetPowerBoxHealth)))

(event Custom|HealthBarUpdate
  ;[1 1 1 1 32] Update Health Bar
  (bind _asoverhead_health_display (Utilities|Casting|CastToOverheadHealthDisplay (UserInterface|GetUserWidgetObject (Variables|Default|GetFloatingHealthBar))))
  (Progress|SetPercent (Variables|/Game/Blueprints/UI_Game/OverheadHealthDisplay.OverheadHealthDisplay_C|GetHealthBar _asoverhead_health_display) (/ (Variables|Default|GetPowerBoxHealth) 1e+02)))

(event Custom|OutOfRangeDamage
  ;[1 1 1 1 32] If Player is out of range - deal damage to player
  (Variables|Default|SetPowerBoxHealth (- (Variables|Default|GetPowerBoxHealth) (Variables|Default|GetDamageOutOfRange)))
  (bind _asthird_person_character (Utilities|Casting|CastToThirdPersonCharacter (Variables|Default|GetOwningPlayer)))
  (Default|ScreenFlash _asthird_person_character))

(event Game|Damage|EventAnyDamage
  (params (Damage :type Float%20%28single-precision%29) (DamageType :type Damage%20Type%20Object%20Reference) (InstigatedBy :type Controller%20Object%20Reference) (DamageCauser :type Actor%20Object%20Reference))
  ;[1 1 1 1 32] Damage Taken
  (if (not (== DamageCauser (Variables|Default|GetOwningPlayer)))
    (Networking|SwitchHasAuthority
      (:Authority
        (bind _output_get (Variables|Default|SetPowerBoxHealth (- (Variables|Default|GetPowerBoxHealth) Damage)))
        (if (<= _output_get 0.0)
          (CallFunction|DeathEvent))))))

(event EventBeginPlay
  ;[1 1 1 1 32] Begin Play
  (CallFunction|HealthBarUpdate)
  (CallFunction|HealthBarRotation)
  (CallFunction|CheckPlayerDistance))

(event Input|KeyboardEvents|F
  (params (Key :type Key%20Structure))
  ;[1 1 1 1 32] Enable Input
  (:Pressed
    (bind _asthird_person_character (Utilities|Casting|CastToThirdPersonCharacter (Variables|Default|GetOwningPlayer)))
    (if (not (Variables|/Game/Blueprints/Characters/ThirdPersonCharacter.ThirdPersonCharacter_C|GetIsInCombat _asthird_person_character))
      (CallFunction|ReturntoPlayer)
      (else
        (Development|PrintString "InCombat!" true true "(R=1.000000,G=0.000000,B=0.000000,A=1.000000)")))))

(fn ConstructionScript
  (Variables|Default|SetOwningPlayer (Components|GetOwner)))

(fn OnRepPowerBoxHealth
  (CallFunction|HealthBarUpdate))