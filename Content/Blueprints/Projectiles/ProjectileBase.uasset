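; Base projectile actor that damages whatever its collision component overlaps and destroys itself after ten seconds if still alive.
; The construction script caches the owner, which is passed as damage causer.
; On overlap, only the authority branch applies damage with the instigator's controller, calls an event that spawns an explosion emitter at the projectile, and destroys the actor.
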(event OnComponentBeginOverlap(ProjectileCollision)
  (params (OverlappedComponent :type Primitive%20Component%20Object%20Reference) (OtherActor :type Actor%20Object%20Reference) (OtherComp :type Primitive%20Component%20Object%20Reference) (OtherBodyIndex :type Integer) (bFromSweep :type Boolean) (SweepResult :type Hit%20Result%20Structure%20%28by%20ref%29))
  ;[1 1 1] Deal Damage
  (Networking|SwitchHasAuthority
    (:Authority
      (Game|Damage|ApplyDamage OtherActor (Variables|Default|GetProjectileDamage) (Game|GetInstigatorController) (Variables|Default|GetOwningPlayerRef) "/Script/Engine.DamageType")
      (CallFunction|MissleEffects)
      (Actor|DestroyActor))))

(event Custom|MissleEffects
  ;[1 1 1] Show Projectile effects
  (Effects|SpawnEmitteratLocation "/Game/Assets/StarterContent/Particles/P_Explosion.P_Explosion" (Transformation|GetWorldLocation (Variables|Default|GetProjectile))))

(event EventBeginPlay
  (Utilities|FlowControl|Delay 1e+01)
  (Actor|DestroyActor))

(fn ConstructionScript
  (Variables|Default|SetOwningPlayerRef (Components|GetOwner)))