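; Bomb is a projectile actor that explodes when its collision component hits something, dealing area damage to pawns.
; On the server, it sphere-overlaps for pawns within an explosion radius and applies damage credited to its instigator's controller.
; It then spawns a scaled explosion emitter, disables collision, hides the mesh and sets a short lifespan for delayed destruction.
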(event OnComponentHit(BombCollision)
  (params (HitComponent :type Primitive%20Component%20Object%20Reference) (OtherActor :type Actor%20Object%20Reference) (OtherComp :type Primitive%20Component%20Object%20Reference) (NormalImpulse :type Vector :default "0, 0, 0") (Hit :type Hit%20Result%20Structure%20%28by%20ref%29))
  (CallFunction|BombDamage))

(event Custom|BombEffects
  ;[1 1 1] Show Bomb effects
  (Effects|SpawnEmitteratLocation "/Game/Assets/StarterContent/Particles/P_Explosion.P_Explosion" (Transformation|GetActorLocation) "0, 0, 0" "5.000000,5.000000,5.000000"))

(event Custom|BombDamage
  ;[1 1 1] Find Actors in explosion radius and apply damage
  (Networking|SwitchHasAuthority
    (:Authority
      (bind _outactors (Collision|SphereOverlapActors (Transformation|GetActorLocation) (Variables|Default|GetExplosionRadius) (Utilities|Array|MakeArray "ObjectTypeQuery3") 0))
      (bind _output_get (Variables|Default|SetHitActors _outactors))
      (for _array_element _output_get
        (Game|Damage|ApplyDamage _array_element (Variables|Default|GetExplosionDamage) (Game|GetInstigatorController) self "/Script/Engine.DamageType"))
      (CallFunction|BombEffects)
      (CallFunction|Hide/DestroyActor))))

(event Custom|Hide/Destroy%20Actor
  (bind _bomb (Variables|Default|GetBomb))
  ;[1 1 1] Destroy Actor with delay
  (Collision|SetCollisionEnabled _bomb "NoCollision")
  (Rendering|SetVisibility _bomb false false)
  (Actor|SetLifeSpan 1.0))

(fn ConstructionScript)