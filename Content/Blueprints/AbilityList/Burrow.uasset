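; Burrow ability Blueprint, currently a debug stub with no burrowing behavior.
; On BeginPlay or BindToEvents, it casts player character 0 to ThirdPersonCharacter and binds its Burrow event to that character's Testing dispatcher, printing success or failure.
; Both the Burrow event and the separate FireAbility event only print debug messages.
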(event Custom|FireAbility
  (Development|PrintString "Burrow Has been fired!"))

(event Custom|BindToEvents
  (bind _asthird_person_character (Utilities|Casting|CastToThirdPersonCharacter (Game|GetPlayerCharacter 0))
    (:then
      (EventDispatchers|BindEventtoTesting _asthird_person_character (delegate Custom|Burrow))
      (Development|PrintString "EventCalled"))
    (:CastFailed
      (Development|PrintString "Fail"))))

(event Custom|Burrow
  (Development|PrintString "WeMadeIt"))

(event EventBeginPlay
  (bind _asthird_person_character (Utilities|Casting|CastToThirdPersonCharacter (Game|GetPlayerCharacter 0))
    (:then
      (EventDispatchers|BindEventtoTesting _asthird_person_character (delegate Custom|Burrow))
      (Development|PrintString "EventCalled"))
    (:CastFailed
      (Development|PrintString "Fail"))))

(fn ConstructionScript
  (|CallParentFunction))