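; Game mode for the main menu that opens the menu when play begins.
; On BeginPlay it casts and stores the GameInstance_Main reference, then calls ShowMainMenu on it, so the game instance owns the menu widget.
; It then sets UI-only input focused on that widget and shows the mouse cursor.
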(event Custom|GetGameInstance
  ;[1 1 1] Get a referance to game instance
  (bind _asgame_instance_main (Utilities|Casting|CastToGameInstance_Main (Game|GetGameInstance)))
  (Variables|Ref|SetGameInstanceRef _asgame_instance_main))

(event Custom|CallShowMainMenu
  (bind _returnvalue (Game|GetPlayerController 0))
  (bind _gameinstanceref (Variables|Ref|GetGameInstanceRef))
  ;[1 1 1] Call show main menu and set input mode
  (Default|ShowMainMenu _gameinstanceref)
  (Input|SetInputModeUIOnly _returnvalue (Variables|/Game/Blueprints/General/GameInstance_Main.GameInstance_Main_C|GetMainMenu _gameinstanceref) "DoNotLock")
  (Variables|/Script/Engine.PlayerController|SetbShowMouseCursor _returnvalue true))

(event EventBeginPlay
  ;[0.4623 0.476 1] Get a ref to game instance and call Main menu
  (CallFunction|GetGameInstance)
  (CallFunction|CallShowMainMenu))

(fn ConstructionScript)