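; Main level game mode that spawns the player's selected character on login and shows the game UI.
; BeginPlay caches GameInstance_Main and binds to its player-actor-changed event, which calls ChangePlayerActor without passing a player.
; ChangePlayerActor unpossesses, calls DestroyActor on the player controller itself, then spawns and possesses the new pawn at that controller's transform.
; A GetPlayerActor event that writes the controller's selection to the game instance is never triggered.
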(event Custom|GetGameInstance
  ;[1 1 1] Get Game Instance
  (bind _asgame_instance_main (Utilities|Casting|CastToGameInstance_Main (Game|GetGameInstance)))
  (Variables|Ref|SetGameInstanceRef _asgame_instance_main))

(event Custom|onPlayerActorChanged
  (params (Player%20Actor :type Actor%20Class%20Reference))
  (CallFunction|ChangePlayerActor Player%20Actor))

(event Custom|Get%20Player%20Actor
  (bind _asmy_player_controller (Utilities|Casting|CastToMyPlayerController (Game|GetPlayerController 0)))
  (Default|SetPlayerActor (Variables|Ref|GetGameInstanceRef) (Variables|/Game/Blueprints/General/MyPlayerController.MyPlayerController_C|GetSelectedActor _asmy_player_controller)))

(event Custom|LoadGameUI
  ;[1 1 1] Show Game UI
  (Default|ShowGameUI (Variables|Ref|GetGameInstanceRef)))

(event EventBeginPlay
  ;[0.4069 0.413 1] Main
  (CallFunction|GetGameInstance)
  (EventDispatchers|BindEventtoPlayerActorChanged (Variables|Ref|GetGameInstanceRef) (delegate Custom|onPlayerActorChanged))
  (CallFunction|LoadGameUI))

(event EventPostLogin
  (params (NewPlayer :type Player%20Controller%20Object%20Reference))
  (CallFunction|GetGameInstance)
  (CallFunction|ChangePlayerActor (Variables|/Game/Blueprints/General/GameInstance_Main.GameInstance_Main_C|GetSelectedCharacter (Variables|Ref|GetGameInstanceRef)) NewPlayer))

(fn ConstructionScript)

(fn GetPlayerActor
  (bind _asmy_player_controller (Utilities|Casting|CastToMyPlayerController (Game|GetPlayerController 0)))
  (return (Variables|/Game/Blueprints/General/MyPlayerController.MyPlayerController_C|GetSelectedActor _asmy_player_controller)))

(fn ChangePlayerActor
  (params (Actor :type Actor%20Class%20Reference) (Player :type Player%20Controller%20Object%20Reference))
  (bind _asmy_player_controller (Utilities|Casting|CastToMyPlayerController Player))
  (Pawn|UnPossess _asmy_player_controller)
  (Actor|DestroyActor _asmy_player_controller)
  (bind _aspawn (Utilities|Casting|CastToPawnClass Actor))
  (bind _returnvalue (Game|SpawnActorfromClass _aspawn (Transformation|GetActorTransform _asmy_player_controller) "Undefined" 0 0))
  (Pawn|Possess _asmy_player_controller _returnvalue))