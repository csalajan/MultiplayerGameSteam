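; Player controller that swaps the player's pawn for the character chosen in the game instance.
; ClientPostLogin reads SelectedCharacter from GameInstance_Main and passes it to RespawnPlayerCharacter.
; That event destroys the controlled pawn, spawns the selected Pawn class at the controller's transform and possesses it.
; SelectActor stores a given actor as SelectedActor through SetPlayerActor and returns it.
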(event Custom|SetPlayerActor
  (params (PlayerActor :type Actor%20Class%20Reference))
  (Variables|Default|SetSelectedActor PlayerActor))

(event Custom|Client%20Post%20Login
  (bind _self self)
  (bind _asgame_instance_main (Utilities|Casting|CastToGameInstance_Main (Game|GetGameInstance)))
  (CallFunction|RespawnPlayerCharacter _self _self (Variables|/Game/Blueprints/General/GameInstance_Main.GameInstance_Main_C|GetSelectedCharacter _asgame_instance_main)))

(event Custom|Respawn%20Player%20Character
  (params (Player%20Controller :type My%20Player%20Controller%20Object%20Reference) (Selected%20Character :type Actor%20Class%20Reference))
  (Actor|DestroyActor (Pawn|GetControlledPawn Player%20Controller))
  (bind _aspawn (Utilities|Casting|CastToPawnClass Selected%20Character))
  (bind _returnvalue (Game|SpawnActorfromClass _aspawn (Transformation|GetActorTransform Player%20Controller) "Undefined" 0 0))
  (Pawn|Possess Player%20Controller _returnvalue))

(event EventBeginPlay)

(event EventTick
  (params (DeltaSeconds :type Float%20%28single-precision%29)))

(fn ConstructionScript)

(fn SelectActor
  (params (Player%20Actor :type Actor%20Class%20Reference))
  (CallFunction|SetPlayerActor Player%20Actor)
  (return Player%20Actor))