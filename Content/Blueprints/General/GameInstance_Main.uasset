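; Game instance that manages menu screens and multiplayer sessions for the game.
; Show events lazily create, cache and display widgets for the main, pause, search, host, character select and in-game UI.
; Character select stores session details, then selection either joins when the server name is "none" or hosts MainLevel as a LAN or Steam listen server.
; Destroying the session returns to the MainMenu level.
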(event Custom|Show%20Search%20Games
  ;[1 1 1] Search For Games Menu
  (Utilities|IsValid (Variables|UserInterface|GetSearchGames)
    (:Is%20Valid
      _)
    (:Is%20Not%20Valid
      (bind _returnvalue (UserInterface|CreateWidget "/Game/Blueprints/UI_Menu/SearchGames.SearchGames_C" (Game|GetPlayerController 0)))
      (bind _output_get (Variables|UserInterface|SetSearchGames _returnvalue))))
  (UserInterface|Viewport|AddtoViewport _output_get 0))

(event Custom|ShowGameUI
  ;[1 1 1] Show InGame UI and set Input mode
  (Utilities|IsValid (Variables|UserInterface|GetInGameUI)
    (:Is%20Valid
      _)
    (:Is%20Not%20Valid
      (bind _returnvalue (UserInterface|CreateWidget "/Game/Blueprints/UI_Game/InGameUI.InGameUI_C" (Game|GetPlayerController 0)))
      (bind _output_get (Variables|UserInterface|SetInGameUI _returnvalue))))
  (UserInterface|Viewport|AddtoViewport _output_get 0)
  (Input|SetInputModeGameOnly (Game|GetPlayerController 0)))

(event Custom|SelectCharacter
  (params (SelectedCharacter :type Actor%20Class%20Reference))
  (bind _servername (Variables|Default|GetServerName))
  (Variables|Default|SetSelectedCharacter SelectedCharacter)
  (Development|PrintString _servername)
  (if (Utilities|Enum|Equal(Enum) _servername "none")
    (Development|PrintString "JOINING")
    (CallFunction|JoinSession (Variables|Default|GetSession))
    (else
      (Development|PrintString "HOSTING")
      (CallFunction|LaunchLobby (Variables|Default|GetSteam?) _servername))))

(event Custom|CharacterSelectMenu
  (params (Session :type Blueprint%20Session%20Result%20Structure) (Server%20Name :type String) (Steam? :type Boolean))
  ;[1 1 1] Character Select Menu
  (Variables|Default|SetSession Session)
  (Variables|Default|SetServerName Server%20Name)
  (Variables|Default|SetSteam? Steam?)
  (Utilities|IsValid (Variables|UserInterface|GetCharacterSelect)
    (:Is%20Valid
      _)
    (:Is%20Not%20Valid
      (bind _returnvalue (UserInterface|CreateWidget "/Game/Blueprints/UI_Menu/CharacterSelect.CharacterSelect_C" (Game|GetPlayerController 0)))
      (bind _output_get (Variables|UserInterface|SetCharacterSelect _returnvalue))))
  (UserInterface|Viewport|AddtoViewport _output_get 0))

(event Custom|ShowMainMenu
  ;[1 1 1] MainMenu
  (Utilities|IsValid (Variables|UserInterface|GetMainMenu)
    (:Is%20Valid
      _)
    (:Is%20Not%20Valid
      (bind _returnvalue (UserInterface|CreateWidget "/Game/Blueprints/UI_Menu/MainMenu.MainMenu_C" (Game|GetPlayerController 0)))
      (bind _output_get (Variables|UserInterface|SetMainMenu _returnvalue))))
  (UserInterface|Viewport|AddtoViewport _output_get 0))

(event Custom|ShowPauseMenu
  ;[1 1 1] Pause Menu
  (Utilities|IsValid (Variables|UserInterface|GetPauseMenu)
    (:Is%20Valid
      _)
    (:Is%20Not%20Valid
      (bind _returnvalue (UserInterface|CreateWidget "/Game/Blueprints/UI_Menu/PauseMenu.PauseMenu_C" (Game|GetPlayerController 0)))
      (bind _output_get (Variables|UserInterface|SetPauseMenu _returnvalue))))
  (UserInterface|Viewport|AddtoViewport _output_get 0))

(event Custom|JoinSession
  (params (session :type Blueprint%20Session%20Result%20Structure))
  ;[1 1 1] Join Session (Set input mode)
  (|JoinSession (Game|GetPlayerController 0) session
    (:OnSuccess
      (CallFunction|ShowGameUI))))

(event Custom|LaunchLobby
  (params (Steam? :type Boolean) (Server%20Name :type String))
  ;[1 1 1] Launch Game (set input mode)
  (Variables|Default|SetSessionName Server%20Name)
  (|Session (Game|GetPlayerController 0) 20 (not Steam?)
    (:OnSuccess
      (Game|OpenLevel(byName) "MainLevel" true "listen")
      (Input|SetInputModeGameOnly (Game|GetPlayerController 0)))))

(event Custom|Destroy%20Session
  (params (Player%20Controller :type Player%20Controller%20Object%20Reference))
  ;[1 1 1] Destroy's the session in progress and loads main menu
  (|DestroySession Player%20Controller
    (:OnSuccess
      (Game|OpenLevel(byName) "MainMenu" true "listen"))))

(event Custom|HostGameMenu
  ;[1 1 1] Host Game Menu
  (Utilities|IsValid (Variables|UserInterface|GetHostGame)
    (:Is%20Valid
      _)
    (:Is%20Not%20Valid
      (bind _returnvalue (UserInterface|CreateWidget "/Game/Blueprints/UI_Menu/HostGame.HostGame_C" (Game|GetPlayerController 0)))
      (bind _output_get (Variables|UserInterface|SetHostGame _returnvalue))))
  (UserInterface|Viewport|AddtoViewport _output_get 0))